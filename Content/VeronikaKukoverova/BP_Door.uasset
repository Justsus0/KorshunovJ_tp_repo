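; BP_Door is a double door that swings open when the player character enters its trigger and closes when they leave.
; Overlap events on the We component filter for BP_PlayerCharacter, then play or reverse a single timeline.
; The timeline's track, scaled by a separate OpengDistans variable for each leaf, drives the relative yaw of Cube3 and Cube2.
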(event `self.we.OnComponentBeginOverlap`
  (params (OverlappedComponent :type "PrimitiveComponent Object Reference") (OtherActor :type "Actor Object Reference") (OtherComp :type "PrimitiveComponent Object Reference") (OtherBodyIndex :type Integer) (bFromSweep :type Boolean) (SweepResult :type "HitResult Structure (by ref)"))
  (cast `/Game/ThirdPerson/Blueprints/BP_PlayerCharacter` OtherActor)
  (bind (_direction `_новая_дорожка_0`) (`Timeline|Шкала времени` :!label _label)
    (:`Update`
      (`SceneComponent.K2_SetRelativeRotation` (`self.Cube3`) (`KismetMathLibrary.MakeRotator` 0.0 0.0 (* `_новая_дорожка_0` (`self.opengDistans`))) false false)
      (`SceneComponent.K2_SetRelativeRotation` (`self.Cube2`) (`KismetMathLibrary.MakeRotator` 0.0 0.0 (* `_новая_дорожка_0` (`self.opengDistans2`))) false false))))

(event `self.we.OnComponentEndOverlap`
  (params (OverlappedComponent :type "PrimitiveComponent Object Reference") (OtherActor :type "Actor Object Reference") (OtherComp :type "PrimitiveComponent Object Reference") (OtherBodyIndex :type Integer))
  (cast `/Game/ThirdPerson/Blueprints/BP_PlayerCharacter` OtherActor)
  (goto _label :!via `Reverse`))

(fn `UserConstructionScript`)